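; BP_DummyTarget is a damageable target dummy actor that shows its remaining health as text above it.
; AnyDamage subtracts incoming damage from Health and destroys the actor once Health reaches zero or below.
; Tick rewrites the TextRender component with the current Health value every frame rather than updating it only on damage.
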(event `self.ReceiveTick`
  (params (DeltaSeconds :type "Float (single-precision)"))
  ; Текст над объектом показывает "100% "HP""
  (`TextRenderComponent.K2_SetText` (`self.TextRender`) (`KismetTextLibrary.Conv_DoubleToText` (`self.Health`) "HalfToEven")))

(event `self.ReceiveAnyDamage`
  (params (Damage :type "Float (single-precision)") (DamageType :type "DamageType Object Reference") (InstigatedBy :type "Controller Object Reference") (DamageCauser :type "Actor Object Reference"))
  ; Урон объекта
  (bind _output_get (set `self.Health` (- (`self.Health`) Damage)))
  ; Унечтожение объекта когда HP <= 0%
  (if (<= _output_get 0.0)
    (`self.K2_DestroyActor`)))

(fn `UserConstructionScript`)