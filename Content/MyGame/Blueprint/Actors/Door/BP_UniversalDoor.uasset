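; BP_UniversalDoor is a door actor that opens when something overlaps its box trigger, as a swing, sliding or vertical door.
; A timeline lerps the door's relative transform toward a target selected by door type from the angle, offset or height variables.
; A FlipFlop on timeline completion toggles IsOpen, so leaving the trigger reverses the timeline only once the door has finished opening.
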(event `self.BoxDoor.OnComponentBeginOverlap`
  (params (OverlappedComponent :type "PrimitiveComponent Object Reference") (OtherActor :type "Actor Object Reference") (OtherComp :type "PrimitiveComponent Object Reference") (OtherBodyIndex :type Integer) (bFromSweep :type Boolean) (SweepResult :type "HitResult Structure (by ref)"))
  (if (not (`self.IsOpen?`))
    (bind (_direction _alpha) (`Timeline|DoorTimeLine` :!label _label) ; Door
      (:`Update`
        (`SceneComponent.K2_SetRelativeTransform` (`self.Door`) (`KismetMathLibrary.TLerp` (`KismetMathLibrary.MakeTransform` (0.0 0.0 0.0)) (select `/Game/MyGame/Blueprint/Database/E_DoorType` (`self.DoorType`) :`NewEnumerator0` (`KismetMathLibrary.MakeTransform` (0.0 0.0 0.0) (`KismetMathLibrary.MakeRotator` 0.0 0.0 (`self.OpenAngle`))) :`NewEnumerator1` (`KismetMathLibrary.Conv_VectorToTransform` (`self.SlideOffse`)) :`NewEnumerator2` (`KismetMathLibrary.Conv_VectorToTransform` (`self.LiftHeight`))) _alpha) false false))
      (:`Finished`
        (bind _isa (`/Engine/EditorBlueprintResources/StandardMacros.FlipFlop`)
          (:`A`
            _)
          (:`B`
            _))
        (set `self.IsOpen?` _isa)))))

(event `self.BoxDoor.OnComponentEndOverlap`
  (params (OverlappedComponent :type "PrimitiveComponent Object Reference") (OtherActor :type "Actor Object Reference") (OtherComp :type "PrimitiveComponent Object Reference") (OtherBodyIndex :type Integer))
  (if (`self.IsOpen?`)
    (goto _label :!via `Reverse`)))

(fn `UserConstructionScript`)