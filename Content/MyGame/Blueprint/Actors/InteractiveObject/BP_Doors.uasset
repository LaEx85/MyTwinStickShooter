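; BP_Doors is an interactive sliding door with a text prompt shown while the player character overlaps its Box trigger.
; The Interac event checks IsClosed to play or reverse a Timeline that lerps the Cube's relative X location.
; When the Timeline finishes, a FlipFlop updates IsClosed so the next interaction can move the door the other way.
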(event `self.Box.OnComponentBeginOverlap`
  (params (OverlappedComponent :type "PrimitiveComponent Object Reference") (OtherActor :type "Actor Object Reference") (OtherComp :type "PrimitiveComponent Object Reference") (OtherBodyIndex :type Integer) (bFromSweep :type Boolean) (SweepResult :type "HitResult Structure (by ref)"))
  ; Проверка дверей на появление текста, только когда игрок подойдет!
  (if (== OtherActor (`GameplayStatics.GetPlayerCharacter` 0))
    ; При приближение к колизии дверей появиться надпись "Press "E" to open". отключить галочку Visible в TextRender
    (`SceneComponent.SetVisibility` (`self.TextRender`) true false)))

(event `self.Box.OnComponentEndOverlap`
  (params (OverlappedComponent :type "PrimitiveComponent Object Reference") (OtherActor :type "Actor Object Reference") (OtherComp :type "PrimitiveComponent Object Reference") (OtherBodyIndex :type Integer))
  (if (== OtherActor (`GameplayStatics.GetPlayerCharacter` 0))
    ; При приближение к колизии дверей появиться надпись "Press "E" to open". отключить галочку Visible в TextRender
    (`SceneComponent.SetVisibility` (`self.TextRender`) false false)))

(event `Open door`
  (bind (_direction _alpha) (`Timeline|Timeline` :!label _label)
    (:`Update`
      ; Если Location то двигается дверь по координатам, если открывается дверь то Rotetion
      (`SceneComponent.K2_SetRelativeLocation` (`self.Cube`) (`KismetMathLibrary.MakeVector` (`KismetMathLibrary.Lerp` 0.0 50.0 _alpha)) false false))
    (:`Finished`
      ; Запоминает открыта ли дверь или нет, для повторного вызова объекта
      (bind _isa (`/Engine/EditorBlueprintResources/StandardMacros.FlipFlop`)
        (:`A`
          _)
        (:`B`
          _))
      (set `self.isClosed?` _isa))))

(event `Closed door`
  (goto _label :!via `Reverse`))

(event `/Game/MyGame/Blueprint/Control/BPI_Interactable.Interac`
  (params (Charecter :type "Character Object Reference"))
  ; Создается BP Интерактивный, и называется Interact в поле функции, открываем Class Setting и в нижней части выбераем наш BPI_Interactian
  (if (`self.isClosed?`)
    (`self.Open door`)
    (else
      (`self.Closed door`))))

(fn `UserConstructionScript`)