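; Base player character for a twin-stick shooter, with world-axis Enhanced Input movement and rotation toward the mouse cursor.
; Tick intersects the cursor ray with a horizontal plane at the actor, then turns control yaw at constant speed.
; Firing spawns the projectile class chosen by keys 1–3 at MuzzlePoint after a short Delay.
; E line-traces ahead to message BPI_Interactable actors; hitscan and shotgun fire graphs are left unconnected.
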(event `self.ReceiveBeginPlay`
  ; Привязка контроллера
  (bind _asplayer_controller (cast `PlayerController` (`self.GetController`)))
  (`EnhancedInputSubsystemInterface.AddMappingContext` (pcsubsystem `EnhancedInputLocalPlayerSubsystem` _asplayer_controller) "/Game/HomeWork4/Blueprint/input/IMC_TwinStickShooterDefault.IMC_TwinStickShooterDefault" 0 (struct)))

(event `EnhancedInput|/Game/HomeWork4/Blueprint/input/IA_Walk`
  (params (ActionValue :type "Vector2D Structure") (ElapsedSeconds :type "Float (double-precision)") (TriggeredSeconds :type "Float (double-precision)") (InputAction :type "InputAction Object Reference" :default "/Game/HomeWork4/Blueprint/input/IA_Walk.IA_Walk"))
  (:`Triggered`
    ; Управление клавишами в определенном положение в мире
    (`self.AddMovementInput` (`KismetMathLibrary.GetRightVector` (struct)) ActionValue_X)
    (`self.AddMovementInput` (`KismetMathLibrary.GetForwardVector` (struct)) ActionValue_Y)))

(event `self.ReceiveTick`
  (params (DeltaSeconds :type "Float (single-precision)"))
  (bind (_worldlocation _worlddirection) (`PlayerController.DeprojectMousePositionToWorld` (`GameplayStatics.GetPlayerController` 0)))
  (bind (_returnvalue_roll _returnvalue_pitch _returnvalue_yaw) (`KismetMathLibrary.BreakRotator` (`KismetMathLibrary.RInterpTo_Constant` (`self.K2_GetActorRotation`) (`KismetMathLibrary.FindLookAtRotation` (`self.K2_GetActorLocation`) (`.Intersection` (`KismetMathLibrary.LinePlaneIntersection_OriginNormal` _worldlocation (+ _worldlocation (* _worlddirection 10000.0)) (`self.K2_GetActorLocation`) (0.0 0.0 1.0)))) (`GameplayStatics.GetWorldDeltaSeconds`) 720.0)))
  (`Controller.SetControlRotation` (`self.GetController`) (`KismetMathLibrary.MakeRotator` 0.0 0.0 _returnvalue_yaw)))

(event `EnhancedInput|/Game/HomeWork4/Blueprint/input/IA_Short`
  (params (ActionValue :type Boolean) (ElapsedSeconds :type "Float (double-precision)") (TriggeredSeconds :type "Float (double-precision)") (InputAction :type "InputAction Object Reference" :default "/Game/HomeWork4/Blueprint/input/IA_Short.IA_Short"))
  (bind (_returnvalue_location _returnvalue_rotation) (`KismetMathLibrary.BreakTransform` (`SceneComponent.K2_GetComponentToWorld` (`self.MuzzlePoint`))))
  ; Стрельба через спаун Актора
  (:`Triggered`
    ;; Задержка для стрельбы
    (`KismetSystemLibrary.Delay` 0.2)
    (`|SpawnActorFromClass` (`self.CurrentProjectileClass`) (`KismetMathLibrary.MakeTransform` _returnvalue_location _returnvalue_rotation) "Undefined" "MultiplyWithRoot" null null)))

(event `Key|E`
  (params (Key :type "Key Structure"))
  (bind _capsulecomponent (`self.CapsuleComponent`))
  (bind _returnvalue (`SceneComponent.K2_GetComponentLocation` _capsulecomponent))
  ; Трейс для активации объектов клавишой Е
  (:`Pressed`
    (bind (_outhit _returnvalue_2) (`KismetSystemLibrary.LineTraceSingle` :`Start` _returnvalue :`End` (+ _returnvalue (* (`SceneComponent.GetForwardVector` _capsulecomponent) 100.0)) :`TraceChannel` "TraceTypeQuery1" :`DrawDebugType` "ForDuration"))
    (if _returnvalue_2
      (bind (_bblockinghit _binitialoverlap _time _distance _location _impactpoint _normal _impactnormal _physmat _hitactor) (`GameplayStatics.BreakHitResult` _outhit))
      (if (`KismetSystemLibrary.DoesImplementInterface` _hitactor "/Game/HomeWork4/Blueprint/Control/BPI_Interactable.BPI_Interactable_C")
        (message `/Game/HomeWork4/Blueprint/Control/BPI_Interactable.Interac` _hitactor self)))))

(event `Key|One`
  (params (Key :type "Key Structure"))
  (:`Pressed`
    (set `self.CurrentProjectileClass` "/Game/HomeWork4/Blueprint/Actors/Weapons/BP_Projectile_Pistol.BP_Projectile_Pistol_C")
    (`KismetSystemLibrary.PrintString` "Pistol")))

(event `Key|Two`
  (params (Key :type "Key Structure"))
  (:`Pressed`
    (set `self.CurrentProjectileClass` "/Game/HomeWork4/Blueprint/Actors/Weapons/BP_Projectile_Rifle.BP_Projectile_Rifle_C")
    (`KismetSystemLibrary.PrintString` "Rifle")))

(event `Key|Three`
  (params (Key :type "Key Structure"))
  (:`Pressed`
    (set `self.CurrentProjectileClass` "/Game/HomeWork4/Blueprint/Actors/Weapons/BP_Projectile_Granade.BP_Projectile_Granade_C")
    (`KismetSystemLibrary.PrintString` "Granade")))

(fn `UserConstructionScript`)