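; AI controller that patrols its pawn between the TargetPoint actors in the level.
; BeginPlay collects the points and starts AI MoveTo; each success updates the index in Ping-pong or Circle mode, waits, then calls MoveToPoint again.
; BeginPlay jumps straight to the move, skipping MoveToPoint's point-count check.
; Disconnected experiments remain for single-point movement, player chasing, random roaming and line-trace steering, with their Tick and custom events empty.
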(event `self.ReceiveTick`
  (params (DeltaSeconds :type "Float (single-precision)"))
  ; Перемещение бота по трейсу, запуск через Event Tick
)

(event `MoveToCharacter`
  ; Бот бегает за игроком, через Event Begin Play + Custom Event (для зацыкливания) ноды крепят к Cast to BP_PlayerCharacter
)

(event `Potrol`
  ; Патрулирование бота по рандомным точкам, работает через Event BeginPlay + Custom Event
)

(event `MoveToPoint`
  ; Патрулирование по TargetPoint
  (if (> (`KismetArrayLibrary.Array_Length` (`self.TargetPointBot`)) 1)
    (`|AIMoveTo` (`self.K2_GetPawn`) (`self.K2_GetActorLocation` (`|GetArrayItem` (stale `self.ReceiveBeginPlay` _output_get) (`self.CurrentIndex`))) null 50.0 :!label _label
      (:`OnSuccess`
        (switch `/Game/HomeWork5/DateBase/E_PatrolBot` "NewEnumerator0"
          (:`NewEnumerator0`
            ; Патрулирование по точкам от одной точке к другой
            (set `self.CurrentIndex` (+ (`self.CurrentIndex`) (`self.DirectionIndex`)))
            (if (or (>= (`self.CurrentIndex`) (- (`KismetArrayLibrary.Array_Length` (`self.TargetPointBot`)) 1)) (<= (`self.CurrentIndex`) 0))
              (set `self.DirectionIndex` (* (`self.DirectionIndex`) -1))
              (`KismetSystemLibrary.Delay` 2.0)
              (`self.MoveToPoint` self)
              (else
                (`KismetSystemLibrary.Delay` 2.0)
                (`self.MoveToPoint` self))))
          (:`NewEnumerator1`
            ; Патрулирование по точкам покругу
            (bind _result (`/Engine/EditorBlueprintResources/StandardMacros.IncrementInt` (`self.CurrentIndex`))
              (:`  `
                (set `self.CurrentIndex` (mod _result (`KismetArrayLibrary.Array_Length` (`self.TargetPointBot`))))
                (`KismetSystemLibrary.Delay` 2.0)
                (`self.MoveToPoint`)))))))))

(event `self.ReceiveBeginPlay`
  ; Патрулирование по TargetPoint
  (bind _outactors (`GameplayStatics.GetAllActorsOfClass` "/Script/Engine.TargetPoint"))
  (bind _output_get (set `self.TargetPointBot` _outactors))
  (goto _label))

(fn `UserConstructionScript`)